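; Bullet actor for a Paper2D game, drawn with a flipbook and fired with a direction on the X and Z axes.
; The construction script uniformly scales the flipbook so the sprite's diameter matches the bullet's Radius.
; InitialiseBulletBP sets the translucent sort priority, then passes the pawn, direction, projectile template and effect with its chances to InitialiseABullet.
; The event graph holds no logic.
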(event `self.ReceiveTick`
  (params (DeltaSeconds :type "Float (single-precision)")))

(fn `initialise_BulletBP`
  (params (pawnRef :type "Pawn Object Reference (by ref)") (effect :type "Array of GameplayEffectSpecHandle Structure (by ref)") (effectChances :type "Array of Float (double-precision)") (directionX :type "Float (double-precision)") (directionZ :type "Float (double-precision)") (sortPriority :type Integer) (finalProjectileTemplate :type "ProjectileTemplate Structure (by ref)"))
  (`PrimitiveComponent.SetTranslucentSortPriority` (`self.PaperFlipbook`) sortPriority)
  (`self.initialise_ABullet` :`pawnRef` pawnRef :`directionX` directionX :`directionZ` directionZ :`bulletData` finalProjectileTemplate :`effect` effect :`effectChances` effectChances))

(fn `UserConstructionScript`
  (locals (spriteDiameter :type "Float (double-precision)" :default 13.0))
  (bind _returnvalue (/ (`self.radius`) (/ (`local.spriteDiameter`) 2.0)))
  (`SceneComponent.SetRelativeScale3D` (`self.PaperFlipbook`) (`KismetMathLibrary.MakeVector` _returnvalue _returnvalue _returnvalue)))