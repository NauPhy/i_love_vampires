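; ExplosiveBulletBP is a projectile that spawns an area-of-effect explosion when it dies.
; The construction script scales its Paper2D flipbook uniformly so the sprite matches the projectile radius.
; An init function forwards pawn, effect, direction, projectile and explosion data to an inherited initializer.
; On BulletDeath it spawns AOEBP at its transform with the explosion radius, finishes that explosion's initialization and destroys itself.
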(event `self.bulletDeath`
  (bind _returnvalue (`|SpawnActorFromClass` "/Game/Items/AOEBP.AOEBP_C" (`self.GetTransform`) "Undefined" "MultiplyWithRoot" null (`self.getExplosionRadius`) null))
  (`self.finishExplosionInitialisation` _returnvalue)
  (`self.K2_DestroyActor`))

(fn `initialiseExplosiveBulletBP`
  (params (pawnRef :type "Pawn Object Reference (by ref)") (effect :type "Array of GameplayEffectSpecHandle Structure") (effectChances :type "Array of Float (double-precision)") (directionX :type "Float (double-precision)") (directionZ :type "Float (double-precision)") (projectileData :type "ProjectileTemplate Structure (by ref)") (explosionData :type "AOETemplate Structure"))
  (`self.initialise_AExplosiveBullet` pawnRef effect directionX directionZ projectileData explosionData effectChances))

(fn `UserConstructionScript`
  (locals (spriteDiameter :type "Float (double-precision)" :default 13.0))
  (bind _returnvalue (/ (`self.projectileRadius`) (/ (`local.spriteDiameter`) 2.0)))
  (`SceneComponent.SetRelativeScale3D` (`self.PaperFlipbook`) (`KismetMathLibrary.MakeVector` _returnvalue _returnvalue _returnvalue)))